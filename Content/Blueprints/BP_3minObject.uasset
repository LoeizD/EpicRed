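; BP_3minObject is a countdown timer actor with a widget component that turns to face the player.
; A timeline played in reverse from its end at BeginPlay serves as the clock.
; Each Tick converts its playback position through timespans into minute, second and millisecond variables, then rotates the actor toward the player character.
; The Milliseconds helper's formatting is unconnected, and the WID_Compteur lookup result goes unused.
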(event `self.ReceiveBeginPlay`
  (`self.MakeCounter`)
  (bind _foundwidgets (`WidgetBlueprintLibrary.GetAllWidgetsOfClass` "/Game/Widget/WID_Compteur.WID_Compteur_C"))
  (cast `/Game/Widget/WID_Compteur` (`KismetArrayLibrary.Array_Get` _foundwidgets)))

(event `self.ReceiveTick`
  (params (DeltaSeconds :type "Float (single-precision)"))
  (bind _returnvalue (`TimelineComponent.GetPlaybackPosition` (`self.CounterTimeline`)))
  (bind _returnvalue_2 (`KismetMathLibrary.GetTotalMilliseconds` (`KismetMathLibrary.FromMilliseconds` _returnvalue)))
  (`self.CounterSetVariables` (`KismetTextLibrary.Conv_IntToText` (`.Hours` (`KismetMathLibrary.BreakTimespan` (`KismetMathLibrary.FromMinutes` _returnvalue))) true 1 2) (`KismetTextLibrary.Conv_IntToText` (`.Seconds` (`KismetMathLibrary.BreakTimespan` (`KismetMathLibrary.FromSeconds` _returnvalue))) true 1 2) (`KismetTextLibrary.Conv_DoubleToText` (* (- _returnvalue_2 (`KismetMathLibrary.Conv_IntToDouble` (`KismetMathLibrary.FTrunc` _returnvalue_2))) 1000.0) "HalfToEven" true 1 3 0 0))
  (`self.FacingPlayer`))

(event `MakeCounter`
  (`Timeline|CounterTimeline` :!via `ReverseFromEnd`))

(fn `CounterSetVariables`
  (params (minutes :type Text) (Secondes :type Text) (Millisecondes :type Text))
  (set `self.Counter Min` minutes)
  (set `self.CounterSec` Secondes)
  (set `self.CounterMS` Millisecondes))

(fn `FacingPlayer`
  (`self.K2_SetActorRotation` (`KismetMathLibrary.FindLookAtRotation` (`SceneComponent.K2_GetComponentLocation` (`self.Widget`)) (`self.K2_GetActorLocation` (`GameplayStatics.GetPlayerCharacter` 0)))))

(fn `UserConstructionScript`)