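; BP_Unicorn is an actor for the UnicornBattle interactive object that moves along the world Y axis and bursts on contact with another unicorn.
; A Move timeline started on BeginPlay drives MoveX, which Tick scales by MoveMulti and adds to the location each frame, without sweep or delta-time scaling.
; When its capsule overlaps another BP_Unicorn, it spawns the P_Unicorn particle effect and destroys itself.
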(event `self.ReceiveBeginPlay`
  (bind (_direction _move_y) (`Timeline|Move` :!via `PlayFromStart`)
    (:`Update`
      (set `self.MoveX` _move_y))))

(event `MakeMove`)

(event `self.ReceiveTick`
  (params (DeltaSeconds :type "Float (single-precision)"))
  (`self.K2_SetActorLocation` (+ (`self.K2_GetActorLocation`) (`KismetMathLibrary.MakeVector` 0.0 (* (`self.MoveX`) (`self.MoveMulti`))))))

(event `self.Capsule.OnComponentBeginOverlap`
  (params (OverlappedComponent :type "PrimitiveComponent Object Reference") (OtherActor :type "Actor Object Reference") (OtherComp :type "PrimitiveComponent Object Reference") (OtherBodyIndex :type Integer) (bFromSweep :type Boolean) (SweepResult :type "HitResult Structure (by ref)"))
  (cast `/Game/InteractiveObjects/UnicornBattle/BP_Unicorn` OtherActor)
  (`GameplayStatics.SpawnEmitterAtLocation` "/Game/InteractiveObjects/UnicornBattle/P_Unicorn.P_Unicorn" (`self.K2_GetActorLocation`))
  (`self.K2_DestroyActor`))

(fn `UserConstructionScript`)