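; BP_UnicornBattle is a spawner actor that keeps sending pairs of opposing BP_Unicorn actors into a unicorn battle.
; A looping timer started on BeginPlay calls Spawn every few seconds, placing one unicorn at a random Y offset on each side of the actor.
; Each pair gets opposite rotations and opposite MoveMulti signs, leaving any movement to BP_Unicorn itself.
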(event `self.ReceiveBeginPlay`
  (`KismetSystemLibrary.K2_SetTimerDelegate` (delegate `Spawn`) 5.0 true))

(event `Spawn`
  (bind _returnvalue (`self.GetTransform`))
  (bind _returnvalue_2 (`self.GetTransform`))
  (bind _returnvalue_3 (`|SpawnActorFromClass` "/Game/InteractiveObjects/UnicornBattle/BP_Unicorn.BP_Unicorn_C" (`KismetMathLibrary.MakeTransform` (`KismetMathLibrary.MakeVector` (.x (.location _returnvalue_2)) (- (.y (.location _returnvalue_2)) (`KismetMathLibrary.RandomFloatInRange` 800.0 1500.0)) (.z (.location _returnvalue_2))) (struct :`Yaw` 90.0)) "Undefined" "OverrideRootScale"))
  (set `/Game/InteractiveObjects/UnicornBattle/BP_Unicorn.MoveMulti` 1.0 _returnvalue_3)
  (bind _returnvalue_4 (`|SpawnActorFromClass` "/Game/InteractiveObjects/UnicornBattle/BP_Unicorn.BP_Unicorn_C" (`KismetMathLibrary.MakeTransform` (`KismetMathLibrary.MakeVector` (.x (.location _returnvalue)) (- (.y (.location _returnvalue)) (`KismetMathLibrary.RandomFloatInRange` -800.0 -1500.0)) (.z (.location _returnvalue))) (struct :`Yaw` -90.0)) "Undefined" "OverrideRootScale"))
  (set `/Game/InteractiveObjects/UnicornBattle/BP_Unicorn.MoveMulti` -1.0 _returnvalue_4))

(fn `UserConstructionScript`)