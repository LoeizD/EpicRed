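; BP_Prawn is a short-lived prawn actor built from static meshes that jitter up and down.
; On BeginPlay it starts a fast looping timer and sets a five-second lifespan, after which it is destroyed.
; The timer's Body event uses a FlipFlop to shift all five mesh components up and back down on alternate calls, faking animation without Tick.
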(event `self.ReceiveBeginPlay`
  (`KismetSystemLibrary.K2_SetTimerDelegate` (delegate `Body`) 0.05 true)
  (`self.SetLifeSpan` 5.0))

(event `Body`
  (bind _staticmesh1 (`self.StaticMesh1`))
  (`/Engine/EditorBlueprintResources/StandardMacros.FlipFlop`
    (:`A`
      (`SceneComponent.K2_AddRelativeLocation` _staticmesh1 (0.0 0.0 5.0) false false)
      (`SceneComponent.K2_AddRelativeLocation` (`self.StaticMesh2`) (0.0 0.0 5.0) false false)
      (`SceneComponent.K2_AddRelativeLocation` (`self.StaticMesh3`) (0.0 0.0 5.0) false false)
      (`SceneComponent.K2_AddRelativeLocation` (`self.StaticMesh4`) (0.0 0.0 5.0) false false)
      (`SceneComponent.K2_AddRelativeLocation` (`self.StaticMesh`) (0.0 0.0 5.0) false false))
    (:`B`
      (`SceneComponent.K2_AddRelativeLocation` _staticmesh1 (0.0 0.0 -5.0) false false)
      (`SceneComponent.K2_AddRelativeLocation` (`self.StaticMesh2`) (0.0 0.0 -5.0) false false)
      (`SceneComponent.K2_AddRelativeLocation` (`self.StaticMesh3`) (0.0 0.0 -5.0) false false)
      (`SceneComponent.K2_AddRelativeLocation` (`self.StaticMesh4`) (0.0 0.0 -5.0) false false)
      (`SceneComponent.K2_AddRelativeLocation` (`self.StaticMesh`) (0.0 0.0 -5.0) false false))))

(fn `UserConstructionScript`)