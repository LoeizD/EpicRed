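; BP_3minObject is a three-minute countdown actor that floats in front of the player with a timer widget.
; On BeginPlay it plays CounterTimeline in reverse from the end, with a Shake event track triggering camera shakes.
; Tick converts playback position into minute, second and millisecond counter variables, using timespan unit shifts.
; Tick also turns it toward the player and moves it ahead of the pawn.
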(event `self.ReceiveBeginPlay`
  (`self.MakeCounter`)
  (bind _foundwidgets (`WidgetBlueprintLibrary.GetAllWidgetsOfClass` "/Game/Widget/WID_Compteur.WID_Compteur_C"))
  (cast `/Game/Widget/WID_Compteur` (`KismetArrayLibrary.Array_Get` _foundwidgets)))

(event `self.ReceiveTick`
  (params (DeltaSeconds :type "Float (single-precision)"))
  (bind _returnvalue (`GameplayStatics.GetPlayerPawn` 0))
  (bind _returnvalue_2 (`TimelineComponent.GetPlaybackPosition` (`self.CounterTimeline`)))
  (bind _returnvalue_3 (`KismetMathLibrary.GetTotalMilliseconds` (`KismetMathLibrary.FromMilliseconds` _returnvalue_2)))
  (`self.CounterSetVariables` (`KismetTextLibrary.Conv_IntToText` (`.Hours` (`KismetMathLibrary.BreakTimespan` (`KismetMathLibrary.FromMinutes` _returnvalue_2))) true 1 2) (`KismetTextLibrary.Conv_IntToText` (`.Seconds` (`KismetMathLibrary.BreakTimespan` (`KismetMathLibrary.FromSeconds` _returnvalue_2))) true 1 2) (`KismetTextLibrary.Conv_DoubleToText` (* (- _returnvalue_3 (`KismetMathLibrary.Conv_IntToDouble` (`KismetMathLibrary.FTrunc` _returnvalue_3))) 1000.0) "HalfToEven" true 1 3 0 0))
  (`self.FacingPlayer`)
  (`self.K2_SetActorLocation` (+ (* (`self.GetActorForwardVector` _returnvalue) 200.0) (`self.K2_GetActorLocation` _returnvalue))))

(event `MakeCounter`
  (`Timeline|CounterTimeline` :!via `ReverseFromEnd`
    (:`shake`
      (`PlayerCameraManager.PlayCameraShake` :`self` (`GameplayStatics.GetPlayerCameraManager` 0) :`ShakeClass` "/Game/Blueprints/CamShake/BP_ShakeCam.BP_ShakeCam_C"))))

(fn `CounterSetVariables`
  (params (minutes :type Text) (Secondes :type Text) (Millisecondes :type Text))
  (set `self.Counter Min` minutes)
  (set `self.CounterSec` Secondes)
  (set `self.CounterMS` Millisecondes))

(fn `FacingPlayer`
  (`self.K2_SetActorRotation` (`KismetMathLibrary.FindLookAtRotation` (`SceneComponent.K2_GetComponentLocation` (`self.Widget`)) (`self.K2_GetActorLocation` (`GameplayStatics.GetPlayerCharacter` 0)))))

(fn `UserConstructionScript`)