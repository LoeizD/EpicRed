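; BP_MacaroniSpawner is an actor that continually spawns macaroni, and occasionally prawns, at its own transform.
; A timer starts on BeginPlay, and each spawn picks a new random delay and resets it, giving irregular intervals.
; A weighted roll heavily favours BP_Macaroni, launched upward with random sideways impulse, while BP_Prawn gets a small fixed nudge.
; BeginPlay also caches the first existing BP_Macaroni, though this graph never reads it.
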(event `Reset Timer`
  (`KismetSystemLibrary.K2_SetTimerDelegate` (delegate `Spawn`) (`self.TImeSpawn`) true :!label _label))

(event `self.ReceiveBeginPlay`
  (bind _outactors (`GameplayStatics.GetAllActorsOfClass` "/Game/InteractiveObjects/Macaroni/BP_Macaroni.BP_Macaroni_C"))
  (set `self.RefMacaroni` (`KismetArrayLibrary.Array_Get` _outactors))
  (goto _label))

(event `Spawn`
  (if (`KismetMathLibrary.RandomBoolWithWeight` 0.9)
    (set `self.TImeSpawn` (`KismetMathLibrary.RandomFloatInRange` 0.1 0.8))
    (bind _returnvalue (`|SpawnActorFromClass` "/Game/InteractiveObjects/Macaroni/BP_Macaroni.BP_Macaroni_C" (`self.GetTransform`) "Undefined" "OverrideRootScale"))
    (`PrimitiveComponent.AddImpulse` (`/Game/InteractiveObjects/Macaroni/BP_Macaroni.Capsule` _returnvalue) (`KismetMathLibrary.MakeVector` (`KismetMathLibrary.RandomFloatInRange` -2000.0 2000.0) (`KismetMathLibrary.RandomFloatInRange` -2000.0 2000.0) (`KismetMathLibrary.RandomFloatInRange` 2000.0 10000.0)) "None" false)
    (`self.Reset Timer`)
    (else
      (set `self.TImeSpawn` (`KismetMathLibrary.RandomFloatInRange` 0.1 0.8))
      (bind _returnvalue_2 (`|SpawnActorFromClass` "/Game/InteractiveObjects/Prawn/BP_Prawn.BP_Prawn_C" (`self.GetTransform`) "Undefined" "OverrideRootScale"))
      (`PrimitiveComponent.AddImpulse` (`/Game/InteractiveObjects/Prawn/BP_Prawn.Capsule` _returnvalue_2) (0.0 10.0 0.0) "None" false)
      (`self.Reset Timer`))))

(fn `UserConstructionScript`)