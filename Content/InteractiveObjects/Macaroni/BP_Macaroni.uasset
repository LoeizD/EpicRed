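; BP_Macaroni is a short-lived macaroni actor among the game's interactive objects, with its own sound and particle effect.
; The construction script creates a dynamic material instance and randomizes its MacaroniColor within warm, low-blue ranges, so instances vary.
; BeginPlay starts the FMOD audio and sets a fixed lifespan of a few seconds.
; EndPlay spawns the P_Macaroni emitter at the capsule's location.
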(event `self.ReceiveBeginPlay`
  (`self.SetLifeSpan` 5.0)
  (`FMODAudioComponent.Play` (`self.FMODAudio`)))

(event `self.ReceiveEndPlay`
  (params (EndPlayReason :type "EEndPlayReason Enum" :default "Destroyed"))
  (`GameplayStatics.SpawnEmitterAtLocation` "/Game/InteractiveObjects/Macaroni/P_Macaroni.P_Macaroni" (`SceneComponent.K2_GetComponentLocation` (`self.Capsule`))))

(fn `UserConstructionScript`
  (`parent.UserConstructionScript`)
  (bind _returnvalue (`PrimitiveComponent.CreateDynamicMaterialInstance` (`self.Macaroni`) 0 "/Game/InteractiveObjects/Macaroni/M_Macaroni_Inst.M_Macaroni_Inst"))
  (`MaterialInstanceDynamic.SetVectorParameterValue` _returnvalue "MacaroniColor" (make `LinearColor` (`KismetMathLibrary.RandomFloatInRange` 0.3 0.9) (`KismetMathLibrary.RandomFloatInRange` 0.3 0.8) (`KismetMathLibrary.RandomFloatInRange` 0.0 0.1) 1.0)))