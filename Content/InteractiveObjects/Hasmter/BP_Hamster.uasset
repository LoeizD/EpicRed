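; Hamster actor that flails randomly, with a physics capsule that hops and tumbles.
; From BeginPlay, an endless short random-delay loop applies impulses along the capsule's up or down axis, sometimes setting single-axis spin.
; Tick procedurally rotates four paws, mirrored left to right, and the head by sampling a sine curve at timeline progress.
; Self-restarting random-length loops for those timelines exist, but no event starts them.
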(event `self.ReceiveTick`
  (params (DeltaSeconds :type "Float (single-precision)"))
  (bind _percentage (`/Game/BP_FunctionLibrary.GetTimeLinePercentage` (`self.PatteX`)))
  (bind _percentage_2 (`/Game/BP_FunctionLibrary.GetTimeLinePercentage` (`self.PatteY`)))
  (bind _percentage_3 (`/Game/BP_FunctionLibrary.GetTimeLinePercentage` (`self.PatteZ`)))
  (bind _percentage_4 (`/Game/BP_FunctionLibrary.GetTimeLinePercentage` (`self.Tete`)))
  (bind _returnvalue (+ 60.0 (* (`CurveFloat.GetFloatValue` (`self.CRV_Sin`) _percentage) 45.0)))
  (bind _returnvalue_2 (+ -20.0 (* (`CurveFloat.GetFloatValue` (`self.CRV_Sin`) _percentage_2) 45.0)))
  (bind _returnvalue_3 (+ -20.0 (* (`CurveFloat.GetFloatValue` (`self.CRV_Sin`) _percentage_3) 60.0)))
  (`SceneComponent.K2_SetRelativeRotation` (`self.AvG`) (`KismetMathLibrary.MakeRotator` _returnvalue _returnvalue_2 _returnvalue_3) false false)
  (`SceneComponent.K2_SetRelativeRotation` (`self.ArG`) (`KismetMathLibrary.MakeRotator` _returnvalue _returnvalue_2 _returnvalue_3) false false)
  (`SceneComponent.K2_SetRelativeRotation` (`self.ArD`) (`KismetMathLibrary.MakeRotator` (* _returnvalue -1.0) _returnvalue_2 (* _returnvalue_3 -1.0)) false false)
  (`SceneComponent.K2_SetRelativeRotation` (`self.AvD`) (`KismetMathLibrary.MakeRotator` (* _returnvalue -1.0) _returnvalue_2 (* _returnvalue_3 -1.0)) false false)
  (`SceneComponent.K2_SetRelativeRotation` (`self.Head`) (`KismetMathLibrary.MakeRotator` 0.0 (+ -10.0 (* (`CurveFloat.GetFloatValue` (`self.CRV_Sin`) _percentage_4) 25.0))) false false))

(event `self.ReceiveBeginPlay`
  (bind _returnvalue (`KismetMathLibrary.RandomFloatInRange` 100.0 300.0))
  (bind _capsule (`self.Capsule`))
  (`KismetSystemLibrary.Delay` (`KismetMathLibrary.RandomFloatInRange` 0.1 0.3) :!label _label)
  (`|ExecutionSequence`
    (:`then_0`
      (`PrimitiveComponent.AddImpulse` _capsule (* (`SceneComponent.GetUpVector` (`self.Capsule`)) (select `bool` (`KismetMathLibrary.RandomBool`) :`false` _returnvalue :`true` (* _returnvalue -1.0))) "None" true)
      (if (`KismetMathLibrary.RandomBoolWithWeight` 0.5)
        (`PrimitiveComponent.SetPhysicsAngularVelocity` _capsule (select `int` (`KismetMathLibrary.RandomIntegerInRange` 0 2) :`0` (`KismetMathLibrary.MakeVector` (`KismetMathLibrary.RandomFloatInRange` -1000.0 1000.0)) :`1` (`KismetMathLibrary.MakeVector` 0.0 (`KismetMathLibrary.RandomFloatInRange` -1000.0 1000.0)) :`2` (`KismetMathLibrary.MakeVector` 0.0 0.0 (`KismetMathLibrary.RandomFloatInRange` -1000.0 1000.0))) false "None")))
    (:`then_1`
      (goto _label))))

(fn `UserConstructionScript`
  (`parent.UserConstructionScript`))