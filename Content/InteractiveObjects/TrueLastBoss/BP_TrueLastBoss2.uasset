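; BP_TrueLastBoss2 is a boss actor that rocks its body component back and forth.
; A looping two-second timer flips a direction flag, and Tick adds a fixed per-frame roll to MoveBOdy in that direction, independent of delta time.
; A one-second jump timer also runs, but its event is empty and the upward capsule impulse is left disconnected, so the boss never jumps.
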(event `self.ReceiveBeginPlay`
  (`KismetSystemLibrary.K2_SetTimerDelegate` (delegate `jump`) 1.0 true)
  (`KismetSystemLibrary.K2_SetTimerDelegate` (delegate `Move`) 2.0 true))

(event `jump`)

(event `Move`
  (`/Engine/EditorBlueprintResources/StandardMacros.FlipFlop`
    (:`A`
      (set `self.MoveYN` false))
    (:`B`
      (set `self.MoveYN` true))))

(event `self.ReceiveTick`
  (params (DeltaSeconds :type "Float (single-precision)"))
  (bind _movebody (`self.MoveBOdy`))
  (if (`self.MoveYN`)
    (`SceneComponent.K2_AddRelativeRotation` _movebody (`KismetMathLibrary.MakeRotator` 0.5) false false)
    (else
      (`SceneComponent.K2_AddRelativeRotation` _movebody (`KismetMathLibrary.MakeRotator` -0.5) false false))))

(fn `UserConstructionScript`)